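; BP_Player is the player pawn, with world-axis movement, mouse-steered rotation, automatic fire and health handling.
; On Tick, when mouse velocity exceeds a deadzone threshold, control rotation interpolates toward the yaw of the mouse's movement direction rather than cursor position.
; Holding Shoot runs a delayed loop that spawns BP_RegularShot at ProjectileSpawn until released.
; AffectHealth calls CalculateHealth, prints the result and destroys the actor on death.
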(event Custom|FireBasicShot
  ;[1 1 1] Shoot
  (if (Variables|Default|GetcanShoot)
    (Game|SpawnActorfromClass "/Game/Meshes/Items/BP_RegularShot.BP_RegularShot_C" (Transformation|GetWorldTransform (Variables|Default|GetProjectileSpawn)) "Undefined" 0 0)))

(event EventBeginPlay
  ;[1 1 1] Show Mouse Cursor
  (Variables|/Script/Engine.PlayerController|SetbShowMouseCursor (Game|GetPlayerController 0) true))

(event EventTick
  (params (DeltaSeconds :type Float%20%28single-precision%29))
  (bind _returnvalue (Game|GetPlayerController 0))
  (bind _returnvalue_2 (CallFunction|GetMouseVelocity))
  ;[1 1 1] Rotation
  (if (CallFunction|IsMouseDeadzone)
    (Pawn|SetControlRotation _returnvalue (Math|Interpolation|RInterpTo (Pawn|GetControlRotation _returnvalue :!class /Script/Engine.Controller) (Math|Rotator|MakeRotator 0.0 0.0 (Class|KismetMathLibrary|DegAtan2 (.x _returnvalue_2) (.y _returnvalue_2))) (Utilities|Time|GetWorldDeltaSeconds) (Variables|Default|GetmouseSmoothing)))))

(event EventAffectHealth
  (params (Delta :type Float%20%28single-precision%29))
  (Class|TopDownShooterCharacter|CalculateHealth Delta)
  (Development|PrintString (Utilities|String|ToString(Float) (Variables|Default|Gethealth)) true true "(R=0.987814,G=0.165301,B=1.000000,A=1.000000)")
  (if (Variables|Default|GetisDead)
    (Actor|DestroyActor)))

(event Input|ActionEvents|InputActionShoot
  (params (Key :type Key%20Structure :default "None"))
  ;[1 1 1] Shoot
  (:Pressed
    (Variables|Default|SetcanShoot true)
    (if (Variables|Default|GetcanShoot) :!label _label
      (CallFunction|FireBasicShot)
      (Utilities|FlowControl|Delay 0.2)
      (goto _label)))
  (:Released
    (Variables|Default|SetcanShoot false)))

(event Input|AxisEvents|InputAxisMoveForward
  (params (AxisValue :type Float%20%28single-precision%29))
  ;[1 1 1] Movement
  (Pawn|Input|AddMovementInput "1.000000, 0, 0" AxisValue false))

(event Input|AxisEvents|InputAxisMoveSide
  (params (AxisValue :type Float%20%28single-precision%29))
  ;[1 1 1] Movement
  (Pawn|Input|AddMovementInput "0.000000,1.000000,0.000000" AxisValue false))

(fn ConstructionScript)

(fn GetMouseVelocity
  (bind _returnvalue (Game|GetPlayerController 0))
  (bind (_deltax _deltay) (Class|PlayerController|GetInputMouseDelta _returnvalue))
  (return (/ (Math|Vector2D|MakeVector2D _deltax _deltay) (Utilities|Time|GetWorldDeltaSeconds))))

(fn IsMouseDeadzone
  (return (> (Math|Vector2D|Vector2DLength (CallFunction|GetMouseVelocity)) (Variables|Default|GetmouseDeadzone))))