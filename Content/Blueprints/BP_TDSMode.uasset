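; BP_TDSMode is the game mode (likely for a top-down shooter), handling setup, enemy spawn timing and player respawn.
; On BeginPlay it adds the kill count widget, shows the mouse cursor and starts a looping timer calling SpawnEnemy on the first BP_EnemySpawner found.
; RespawnPlayer spawns a BP_Player at PlayerSpawnPoint and possesses it with player controller 0.
; The construction script applies windowed mode at a fixed resolution.
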(event Custom|RespawnPlayer
  ;[1 1 1] Respawn Player
  (bind _returnvalue (Game|SpawnActorfromClass "/Game/Blueprints/BP_Player.BP_Player_C" (Variables|Default|GetPlayerSpawnPoint) "Undefined" 0 0))
  (Pawn|Possess (Game|GetPlayerController 0) _returnvalue))

(event EventBeginPlay
  ;[1 1 1] Show Mouse Cursor
  (Utilities|FlowControl|Sequence
    (:then_0
      (bind _returnvalue (UserInterface|CreateWidget "/Game/Blueprints/Widget_KillCount.Widget_KillCount_C"))
      (UserInterface|Viewport|AddtoViewport _returnvalue 0))
    (:then_1
      (Variables|/Script/Engine.PlayerController|SetbShowMouseCursor (Game|GetPlayerController 0) true)
      ;[1 1 1] Spawn Enemies
      (bind _outactors (Actor|GetAllActorsOfClass "/Game/Blueprints/BP_EnemySpawner.BP_EnemySpawner_C"))
      (bind _output_get (Variables|Default|SetSpawner (Utilities|Array|Get(acopy) _outactors)))
      (Utilities|Time|SetTimerbyFunctionName _output_get "SpawnEnemy" (Variables|Default|GetspawnTime) true))))

(fn ConstructionScript
  (bind _returnvalue (Settings|GetGameUserSettings))
  (Utilities|FlowControl|Sequence
    (:then_0
      (Class|GameUserSettings|SetFullscreenMode _returnvalue "Windowed"))
    (:then_1
      (Class|GameUserSettings|SetScreenResolution _returnvalue (Utilities|Struct|MakeIntPoint 1280 720)))
    (:then_2
      (Class|GameUserSettings|ApplySettings _returnvalue true))))